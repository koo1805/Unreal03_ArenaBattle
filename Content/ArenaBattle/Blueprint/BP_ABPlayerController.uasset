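; BP_ABPlayerController is the ArenaBattle player controller that owns the on-screen HUD and the end-of-game result screen.
; On BeginPlay it creates the HUD widget, keeps its player score sub-widget and fills in the clear-score target from the game mode.
; Score and retry-count events update that score widget, while game-over and game-clear events each spawn a result widget showing failure or success.
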(event EventOnGameRetryCount
  (params (NewRetryCount :type Integer))
  ;[0.0288 0.04182 0.15 0.5] 재시도 횟수 설정
  (Default|SetRetryCount (Variables|Default|GetScoreWidget) NewRetryCount))

(event EventOnScoreChanged
  (params (NewScore :type Integer))
  (Default|SetScore (Variables|Default|GetScoreWidget) NewScore))

(event EventOnGameClear
  (Variables|Default|SetIsSuccess true)
  (bind _returnvalue (UserInterface|CreateWidget "/Game/ArenaBattle/UI/WBP_GameResult.WBP_GameResult_C"))
  (UserInterface|Viewport|AddtoViewport _returnvalue 0)
  (Default|SetResult _returnvalue (Variables|Default|GetIsSuccess)))

(event EventOnGameOver
  (Variables|Default|SetIsSuccess false)
  (bind _returnvalue (UserInterface|CreateWidget "/Game/ArenaBattle/UI/WBP_GameResult.WBP_GameResult_C"))
  (UserInterface|Viewport|AddtoViewport _returnvalue 0)
  (Default|SetResult _returnvalue (Variables|Default|GetIsSuccess)))

(event EventBeginPlay
  (bind _returnvalue (UserInterface|CreateWidget "/Game/ArenaBattle/UI/WBP_ABHUD.WBP_ABHUD_C"))
  (bind _output_get (Variables|Default|SetABHUDWidget _returnvalue))
  (UserInterface|Viewport|AddtoViewport _output_get 0)
  (bind _output_get_2 (Variables|Default|SetScoreWidget (Variables|/Game/ArenaBattle/UI/WBP_ABHUD.WBP_ABHUD_C|GetWBP_PlayerScore _returnvalue)))
  (bind _returnvalue_2 (Class|ABGameInterface|GetClearScore(Message) (Game|GetGameMode)))
  (Default|SetClearScore _output_get_2 _returnvalue_2))

(fn ConstructionScript)